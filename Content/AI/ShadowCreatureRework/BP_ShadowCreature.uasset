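; Shadow creature AI Blueprint that provides a melee attack and a spell attack.
; The melee event plays a montage on the main mesh.
; The spell event spawns a ShadowDeath effect and a Spell_Base actor at SpellPoint, then destroys that actor after a short delay.
; The construction script makes ShadowCreatureShell follow the main mesh's animation through leader pose.
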(event Custom|MeleeAttack_1
  (Animation|Montage|PlayMontage (Variables|Character|GetMesh) 0))

(event EventSpellAttack
  (bind _spellpoint (Variables|Default|GetSpellPoint))
  (bind _returnvalue (Transformation|GetWorldTransform _spellpoint))
  (Niagara|SpawnSystematLocation "/Game/PC/SpellBook/Spells/Niagara/ShadowDeath.ShadowDeath" (.location _returnvalue) (.rotation _returnvalue))
  (bind _returnvalue_2 (Game|SpawnActorfromClass "/Game/PC/SpellBook/Spell_Base.Spell_Base_C" (Math|Transform|MakeTransform (.location _returnvalue) (.rotation _returnvalue) "1.000000,1.000000,1.000000") "AlwaysSpawn" 0 0 0))
  (Utilities|FlowControl|Delay 3.0)
  (Actor|DestroyActor _returnvalue_2))

(fn ConstructionScript
  (Components|SkinnedMesh|SetLeaderPoseComponent (Variables|Default|GetShadowCreature_Shell) (Variables|Character|GetMesh) false false))