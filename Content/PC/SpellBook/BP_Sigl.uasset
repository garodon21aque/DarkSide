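; BP_Sigl is a sigil actor that acts as a trap for BP_ShadowCreature.
; When a shadow creature overlaps it, the sigil plays the creature's trapped montage and disables its movement.
; After a fixed delay it restores walking movement and destroys itself, so each sigil is single-use.
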(event EventBeginPlay)

(event Collision|EventActorBeginOverlap
  (params (OtherActor :type Actor%20Object%20Reference))
  (bind _asbp_shadow_creature (Utilities|Casting|CastToBP_ShadowCreature OtherActor))
  (bind _output_get (Variables|Default|SetAs%20BP%20Shadow%20Creature_0 _asbp_shadow_creature))
  (Utilities|IsValid _output_get
    (:Is%20Valid
      (Animation|PlayAnimMontage _output_get "/Game/Assets/Assets/Shadow_Dog/Extra/ShadowCreature_Anim_RIG-ArmatureEar_L_Shadow_Trapped_Montage.ShadowCreature_Anim_RIG-ArmatureEar_L_Shadow_Trapped_Montage" 1.0 "None")
      (Pawn|Components|CharacterMovement|DisableMovement (Variables|/Script/Engine.Character|GetCharacterMovement _output_get))
      (Utilities|FlowControl|Delay 1e+01)
      (Pawn|Components|CharacterMovement|SetMovementMode (Variables|/Script/Engine.Character|GetCharacterMovement _output_get) "MOVE_Walking" 0)
      (Actor|DestroyActor))))

(event EventTick
  (params (DeltaSeconds :type Float%20%28single-precision%29)))

(fn ConstructionScript)