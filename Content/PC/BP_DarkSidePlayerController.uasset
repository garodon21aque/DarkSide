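; BP_DarkSidePlayerController is a player controller that creates and refreshes the HUD and keeps a world timer.
; BeginPlay starts a looping one-second timer, then adds the HUD to the viewport, passing it light values and a character reference.
; Each tick of that timer increments WorldTimer, casts player 0's character to BP_DarkSideCharacter and updates the HUD.
; That cast first runs in the timer, after BeginPlay has already read the character reference.
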(event Custom|Timer
  (bind _result (Math|Float|IncrementFloat (Variables|Default|GetWorldTimer))
    (:%20%20
      (Variables|Default|SetWorldTimer _result)
      (bind _asbp_dark_side_character (Utilities|Casting|CastToBP_DarkSideCharacter (Game|GetPlayerCharacter 0)))
      (Default|Update (stale EventBeginPlay _output_get)))))

(event EventBeginPlay
  (Utilities|Time|SetTimerbyEvent (delegate Custom|Timer) 1.0 true)
  (bind _returnvalue (UserInterface|CreateWidget "/Game/UI/HUD/HUD.HUD_C" 0 (Variables|/Game/PC/BP_DarkSideCharacter.BP_DarkSideCharacter_C|GetActive%20Lights (stale Custom|Timer _asbp_dark_side_character)) (Variables|/Game/PC/BP_DarkSideCharacter.BP_DarkSideCharacter_C|GetMax%20Light (stale Custom|Timer _asbp_dark_side_character)) 0.0 0 (stale Custom|Timer _asbp_dark_side_character)))
  (bind _output_get (Variables|Default|SetHud _returnvalue))
  (UserInterface|Viewport|AddtoViewport _returnvalue 0))

(event EventTick
  (params (DeltaSeconds :type Float%20%28single-precision%29)))

(fn ConstructionScript)