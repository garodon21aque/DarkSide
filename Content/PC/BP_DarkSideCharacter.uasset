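; Player character for the Dark Side game, casting spells that use Health as their resource.
; Inputs fire a projectile that destroys shadow creatures, spawn a sigil, or raise a timed barrier; creature contact drains Health, while barrier contact restores it after a delay.
; Looping timers poll for death, which disables movement, plays a montage and quits, and copy light counts from overlapping BP_Level actors.
; The Aura mesh follows the body via leader pose.
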(event OnComponentBeginOverlap(Barrier)
  (params (OverlappedComponent :type Primitive%20Component%20Object%20Reference) (OtherActor :type Actor%20Object%20Reference) (OtherComp :type Primitive%20Component%20Object%20Reference) (OtherBodyIndex :type Integer) (bFromSweep :type Boolean) (SweepResult :type Hit%20Result%20Structure%20%28by%20ref%29))
  (bind _playerattributes (Variables|Default|GetPlayerAttributes))
  (Utilities|Casting|CastToBP_ShadowCreature OtherActor)
  (Utilities|FlowControl|Delay 1e+01)
  (Variables|/Script/DarkSide.AttributeComponent|SetHealth _playerattributes (Variables|/Script/DarkSide.AttributeComponent|GetMaxHealth _playerattributes)))

(event OnComponentBeginOverlap(CapsuleComponent)
  (params (OverlappedComponent :type Primitive%20Component%20Object%20Reference) (OtherActor :type Actor%20Object%20Reference) (OtherComp :type Primitive%20Component%20Object%20Reference) (OtherBodyIndex :type Integer) (bFromSweep :type Boolean) (SweepResult :type Hit%20Result%20Structure%20%28by%20ref%29))
  (bind _playerattributes (Variables|Default|GetPlayerAttributes))
  (Utilities|Casting|CastToBP_ShadowCreature OtherActor)
  (Variables|/Script/DarkSide.AttributeComponent|SetHealth _playerattributes (- (Variables|/Script/DarkSide.AttributeComponent|GetHealth _playerattributes) 5.0)))

(event Custom|OnActorBeginOverlap_Event
  (params (OverlappedActor :type Actor%20Object%20Reference) (OtherActor :type Actor%20Object%20Reference))
  (bind _asbp_shadow_creature (Utilities|Casting|CastToBP_ShadowCreature OtherActor))
  (Utilities|IsValid _asbp_shadow_creature
    (:Is%20Valid
      (Actor|DestroyActor _asbp_shadow_creature)
      (Niagara|SpawnSystematLocation "/Game/PC/SpellBook/Spells/Niagara/ShadowDeath.ShadowDeath" (Transformation|GetWorldLocation (Variables|/Script/Engine.Character|GetMesh _asbp_shadow_creature)))
      (Actor|DestroyActor (stale Input|ActionEvents|InputActionBind _returnvalue_2)))))

(event Custom|Death
  (if (<= (Variables|/Script/DarkSide.AttributeComponent|GetHealth (Variables|Default|GetPlayerAttributes)) 0.0)
    (Pawn|Components|CharacterMovement|DisableMovement (Variables|Character|GetCharacterMovement))
    (Utilities|FlowControl|DoOnce false
      (:Completed
        (Animation|Montage|PlayMontage (Variables|Character|GetMesh) "/Game/Assets/3D_Assets/PC_Assets/PC_Death_Montage.PC_Death_Montage" 2.0
          (:then
            _)
          (:OnCompleted
            (Physics|SetSimulatePhysics (Variables|Character|GetMesh) true)))
        (Rendering|Material|SetMaterial (Variables|Default|GetAura) 0 "/Game/Assets/3D_Assets/PC_Aura_Instance.PC_Aura_Instance")
        (Utilities|FlowControl|Delay 3.0)
        (Game|QuitGame 0 "Quit" false)))))

(event Custom|BP_LevelChecker
  (for _array_element (Collision|GetOverlappingActors (Variables|Character|GetMesh) "/Game/Assets/BluePrints/BP_Level.BP_Level_C" :!class /Script/Engine.PrimitiveComponent)
    (Utilities|IsValid _array_element
      (:Is%20Valid
        (bind _asbp_level (Utilities|Casting|CastToBP_Level _array_element))
        (Utilities|IsValid _asbp_level
          (:Is%20Valid
            (Variables|Default|SetActive%20Lights (Variables|/Game/Assets/BluePrints/BP_Level.BP_Level_C|GetActiveLights _asbp_level))
            (Variables|Default|SetMax%20Light (Variables|/Game/Assets/BluePrints/BP_Level.BP_Level_C|GetMaxLight _asbp_level))))))))

(event EventBeginPlay
  (Collision|SetCollisionEnabled (Variables|Default|GetBarrier) "NoCollision")
  (Utilities|Time|SetTimerbyEvent (delegate Custom|Death) 2.0 true)
  (Utilities|Time|SetTimerbyEvent (delegate Custom|BP_LevelChecker) 2.0 true))

(event Collision|EventActorBeginOverlap
  (params (OtherActor :type Actor%20Object%20Reference)))

(event EventTick
  (params (DeltaSeconds :type Float%20%28single-precision%29)))

(event Input|ActionEvents|InputActionBarrier
  (params (Key :type Key%20Structure :default "None"))
  (bind _playerattributes (Variables|Default|GetPlayerAttributes))
  (:Pressed
    (if (not (< (Variables|/Script/DarkSide.AttributeComponent|GetHealth _playerattributes) 8e+01))
      (if (not (<= (Variables|/Script/DarkSide.AttributeComponent|GetHealth _playerattributes) (- (Variables|/Script/DarkSide.AttributeComponent|GetHealth _playerattributes) 8e+01)))
        (bind _output_get (Variables|/Script/DarkSide.AttributeComponent|SetHealth _playerattributes (- (Variables|/Script/DarkSide.AttributeComponent|GetHealth _playerattributes) 8e+01)))
        (Development|PrintString (Utilities|String|ToString(Float) _output_get))
        (Collision|SetCollisionEnabled (Variables|Default|GetBarrier) "QueryAndPhysics")
        (Rendering|SetVisibility (Variables|Default|GetBarrier%20Spell) true false)
        (Rendering|SetVisibility (Variables|Default|GetStaticMesh) true false)
        (Utilities|FlowControl|Delay 5.0)
        (Rendering|SetVisibility (Variables|Default|GetBarrier%20Spell) false false)
        (Rendering|SetVisibility (Variables|Default|GetStaticMesh) false false)
        (Collision|SetCollisionEnabled (Variables|Default|GetBarrier) "NoCollision")))))

(event Input|ActionEvents|InputActionBind
  (params (Key :type Key%20Structure :default "None"))
  (bind _playerattributes (Variables|Default|GetPlayerAttributes))
  (bind _arrow1 (Variables|Default|GetArrow1))
  (bind _returnvalue (Transformation|GetWorldTransform _arrow1))
  (:Pressed
    (if (not (< (Variables|/Script/DarkSide.AttributeComponent|GetHealth _playerattributes) 2e+01))
      (Utilities|Casting|CastToBP_DarkSidePlayerController (Game|GetPlayerController 0))
      (Variables|/Script/DarkSide.AttributeComponent|SetHealth _playerattributes (- (Variables|/Script/DarkSide.AttributeComponent|GetHealth _playerattributes) 1e+01))
      (bind _returnvalue_2 (Game|SpawnActorfromClass "/Game/PC/SpellBook/Spell_Base.Spell_Base_C" (Math|Transform|MakeTransform (.location _returnvalue) (Math|Rotator|MakeRotator (.roll (.rotation _returnvalue)) (.pitch (.rotation _returnvalue)) (.yaw (.rotation _returnvalue))) (.scale _returnvalue)) "AlwaysSpawn" 0 0))
      (EventDispatchers|AssignOnActorBeginOverlap _returnvalue_2 (delegate Custom|OnActorBeginOverlap_Event))
      (Utilities|FlowControl|Delay 4.0)
      (Actor|DestroyActor _returnvalue_2))))

(event Input|ActionEvents|InputActionWall
  (params (Key :type Key%20Structure :default "None"))
  (bind _mesh (Variables|Character|GetMesh))
  (bind _returnvalue (Transformation|GetWorldTransform _mesh))
  (:Pressed
    (Game|SpawnActorfromClass "/Game/PC/SpellBook/BP_Sigl.BP_Sigl_C" (Math|Transform|MakeTransform (+ (.location _returnvalue) "50.000000,0.000000,0.000000") (.rotation _returnvalue) "1.000000,1.000000,1.000000") "Undefined" 0 0)))

(fn ConstructionScript
  (Components|SkinnedMesh|SetLeaderPoseComponent (Variables|Default|GetAura) (Variables|Character|GetMesh) true false))