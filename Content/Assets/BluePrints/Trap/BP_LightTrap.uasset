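; BP_LightTrap is a trap that damages the player and spawns shadow creatures while its spotlight is active.
; Overlapping Trap_Set with BP_DarkSideCharacter applies one-time damage and lights the spotlight.
; A looping timer prunes invalid enemies and refills the array to MaxEnemy at EnemySpawn.
; A creature leaving Trap_Finish destroys the first array entry; the player-exit light shutoff is chained behind that creature cast, using the same actor.
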(event OnComponentBeginOverlap(Trap_Set)
  (params (OverlappedComponent :type Primitive%20Component%20Object%20Reference) (OtherActor :type Actor%20Object%20Reference) (OtherComp :type Primitive%20Component%20Object%20Reference) (OtherBodyIndex :type Integer) (bFromSweep :type Boolean) (SweepResult :type Hit%20Result%20Structure%20%28by%20ref%29))
  (bind _asbp_dark_side_character (Utilities|Casting|CastToBP_DarkSideCharacter OtherActor))
  (bind _output_get (Variables|Default|SetPc _asbp_dark_side_character))
  (Utilities|FlowControl|DoOnce false
    (:Completed
      (Variables|/Script/DarkSide.AttributeComponent|SetHealth (Variables|/Script/DarkSide.DarkSideCharacter|GetPlayerAttributes _output_get) (- (Variables|/Script/DarkSide.AttributeComponent|GetHealth (Variables|/Script/DarkSide.DarkSideCharacter|GetPlayerAttributes _output_get)) 2e+01))
      (Rendering|Components|Light|SetIntensity (Variables|Default|GetSpotLight) 5e+03)
      (Components|Activation|Activate (Variables|Default|GetSpotLight) false))))

(event OnComponentEndOverlap(Trap_Finish)
  (params (OverlappedComponent :type Primitive%20Component%20Object%20Reference) (OtherActor :type Actor%20Object%20Reference) (OtherComp :type Primitive%20Component%20Object%20Reference) (OtherBodyIndex :type Integer))
  (bind _spotlight (Variables|Default|GetSpotLight))
  (bind _asbp_shadow_creature (Utilities|Casting|CastToBP_ShadowCreature OtherActor))
  (Variables|Default|SetAs%20BP%20Shadow%20Creature _asbp_shadow_creature)
  (Actor|DestroyActor (Utilities|Array|Get(acopy) (Variables|Default|GetEnemy)))
  (bind _asbp_dark_side_character (Utilities|Casting|CastToBP_DarkSideCharacter OtherActor))
  (Utilities|IsValid _asbp_dark_side_character
    (:Is%20Valid
      (Rendering|Components|Light|SetIntensity _spotlight 0.0)
      (Components|Activation|Deactivate _spotlight))))

(event Custom|ChekcingEnemy
  (bind _enemy (Variables|Default|GetEnemy))
  (bind (_arrayindex _arrayelement) (Utilities|Array|ReverseforEachLoop _enemy)
    (:LoopBody
      (Utilities|IsValid _arrayelement
        (:Is%20Not%20Valid
          (Utilities|Array|RemoveIndex _enemy _arrayindex))))
    (:Completed
      (CallFunction|RespawnEnemy))))

(event Custom|RespawnEnemy
  (bind _enemy (Variables|Default|GetEnemy))
  (bind _maxenemy (Variables|Default|GetMaxEnemy))
  (bind _enemyspawn (Variables|Default|GetEnemySpawn))
  (bind _returnvalue (Utilities|Array|Length _enemy))
  (bind _returnvalue_2 (Transformation|GetWorldTransform _enemyspawn))
  (if (< _returnvalue _maxenemy)
    (if (Components|Activation|IsActive (Variables|Default|GetSpotLight))
      (for _index (range 1 (- _maxenemy _returnvalue))
        (bind _returnvalue_3 (Game|SpawnActorfromClass "/Game/AI/ShadowCreatureRework/BP_ShadowCreature.BP_ShadowCreature_C" (Math|Transform|MakeTransform (.location _returnvalue_2) (.rotation _returnvalue_2) "1.000000,1.000000,1.000000") "AlwaysSpawn" 0 0))
        (Utilities|Array|Add (Variables|Default|GetEnemy) _returnvalue_3)))))

(event EventBeginPlay
  (Utilities|Time|SetTimerbyEvent (delegate Custom|ChekcingEnemy) 5.0 true))

(event Collision|EventActorBeginOverlap
  (params (OtherActor :type Actor%20Object%20Reference)))

(event EventTick
  (params (DeltaSeconds :type Float%20%28single-precision%29)))

(fn ConstructionScript)