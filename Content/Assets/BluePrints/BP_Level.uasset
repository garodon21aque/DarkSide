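; BP_Level is a level-section actor that tracks shadow spawner lights inside its LightSources volume and completes when none remain active.
; Player overlap activates it and updates the character's light counters, while CheckingLight recounts active spawners.
; FinishedLevel destroys all light creatures and marks completion; OpenLevel's polling timer is unconnected.
; SpawnLightCreature spawns a creature at a random reachable point around the active light nearest the switched-off one.
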(event OnComponentBeginOverlap(LightSources)
  (params (OverlappedComponent :type Primitive%20Component%20Object%20Reference) (OtherActor :type Actor%20Object%20Reference) (OtherComp :type Primitive%20Component%20Object%20Reference) (OtherBodyIndex :type Integer) (bFromSweep :type Boolean) (SweepResult :type Hit%20Result%20Structure%20%28by%20ref%29))
  (bind _defaultsceneroot (Variables|Default|GetDefaultSceneRoot))
  (bind _light_sources (Variables|Default|GetLight%20Sources))
  (bind _overlappingactors (Collision|GetOverlappingActors _light_sources "/Game/AI/BP_ShadowSpawner.BP_ShadowSpawner_C" :!class /Script/Engine.PrimitiveComponent))
  (bind _asbp_dark_side_character (Utilities|Casting|CastToBP_DarkSideCharacter (Utilities|Array|Get(acopy) (Collision|GetOverlappingActors (Variables|Default|GetLight%20Sources) "/Game/PC/BP_DarkSideCharacter.BP_DarkSideCharacter_C" :!class /Script/Engine.PrimitiveComponent))))
  (Utilities|IsValid _asbp_dark_side_character
    (:Is%20Valid
      (Components|Activation|SetActive _defaultsceneroot true false)
      (if (Components|Activation|IsActive _defaultsceneroot)
        (for _array_element _overlappingactors
          (bind _returnvalue (Utilities|Array|Add _overlappingactors _array_element))
          (Variables|/Game/PC/BP_DarkSideCharacter.BP_DarkSideCharacter_C|SetMax%20Light _asbp_dark_side_character _returnvalue)
          (bind _asbp_shadow_spawner (Utilities|Casting|CastToBP_ShadowSpawner _array_element))
          (Development|PrintString (Utilities|String|ToString(Boolean) (Variables|/Game/AI/BP_ShadowSpawner.BP_ShadowSpawner_C|GetIsActive _asbp_shadow_spawner)))
          (if (not (Variables|/Game/AI/BP_ShadowSpawner.BP_ShadowSpawner_C|GetIsActive _asbp_shadow_spawner))
            (Variables|/Game/PC/BP_DarkSideCharacter.BP_DarkSideCharacter_C|SetActive%20Lights _asbp_dark_side_character 0)))))))

(event Custom|Checking%20Light
  (bind _lights (Variables|Default|GetLights))
  (Utilities|Array|Clear (Variables|Default|GetLights))
  (for _array_element (Collision|GetOverlappingActors (Variables|Default|GetLight%20Sources) "/Game/AI/BP_ShadowSpawner.BP_ShadowSpawner_C" :!class /Script/Engine.PrimitiveComponent)
    (bind _asbp_shadow_spawner (Utilities|Casting|CastToBP_ShadowSpawner _array_element))
    (Utilities|Array|Add _lights _asbp_shadow_spawner))
  (Variables|Default|SetActiveLights 0)
  (for _array_element_2 _lights
    (bind _asbp_shadow_spawner_2 (Utilities|Casting|CastToBP_ShadowSpawner _array_element_2))
    (if (Variables|/Game/AI/BP_ShadowSpawner.BP_ShadowSpawner_C|GetIsActive _asbp_shadow_spawner_2)
      (Variables|Default|SetActiveLights (+ (Variables|Default|GetActiveLights) 1)))))

(event Custom|Open%20Level
  (if (not (Components|Activation|IsActive (Variables|Default|GetDefaultSceneRoot)))
    (for _index (range 0 (+ (Utilities|Array|Length (Variables|Default|GetLights)) 1))
      (Variables|Default|SetMaxLight (+ _index -1))
      (CallFunction|FinishedLevel))))

(event Custom|Finished%20Level
  (if (== (Variables|Default|GetActiveLights) 0)
    (bind _outactors (Actor|GetAllActorsOfClass "/Game/AI/LightCreature/BP_LightCreature.BP_LightCreature_C"))
    (for _array_element _outactors
      (Actor|DestroyActor _array_element)
      (Components|Activation|Deactivate (Variables|Default|GetDefaultSceneRoot))
      (Variables|Default|SetIsCompleted true)
      (bind _result (Math|Integer|IncrementInt (Variables|Default|GetCompleted))
        (:%20%20
          (Variables|Default|SetCompleted _result)
          (Collision|SetCollisionResponsetoAllChannels (Variables|Default|GetLight%20Sources) "ECR_Overlap"))))))

(event EventBeginPlay)

(fn ConstructionScript)

(fn SpawnLightCreature
  (params (SwitchedOffLightPos :type Vector) (LevelReference :type BP%20Level%20Object%20Reference))
  (Variables|Default|SetDistanceForSpawningLightCreature 999999999999.0)
  (for _array_element (Variables|Default|GetLights)
    (bind _asbp_shadow_spawner (Utilities|Casting|CastToBP_ShadowSpawner _array_element))
    (if (Variables|/Game/AI/BP_ShadowSpawner.BP_ShadowSpawner_C|GetIsActive _asbp_shadow_spawner)
      (if (<= (Math|Vector|Distance(Vector) (Transformation|GetActorLocation _array_element) SwitchedOffLightPos) (Variables|Default|GetDistanceForSpawningLightCreature))
        (Variables|Default|SetDistanceForSpawningLightCreature (Math|Vector|Distance(Vector) (Transformation|GetActorLocation _array_element) SwitchedOffLightPos))
        (Variables|Default|SetLightCreatureSpawnPos (Transformation|GetActorLocation _array_element)))))
  (if (> (Variables|Default|GetActiveLights) 0)
    (bind _returnvalue (Game|SpawnActorfromClass "/Game/AI/LightCreature/BP_LightCreature.BP_LightCreature_C" (Math|Transform|MakeTransform (.RandomLocation (AI|Navigation|GetRandomReachablePointinRadius (Variables|Default|GetLightCreatureSpawnPos) (Math|Float|Clamp(Float) (Math|Random|RandomFloat) 2e+02 4e+02) 0 0)) "0, 0, 0" "1.000000,1.000000,1.000000") "AdjustIfPossibleButAlwaysSpawn" 0 0 2 false 0))
    (bind _output_get (Variables|Default|SetLightCreature _returnvalue))
    (Variables|/Game/AI/LightCreature/BP_LightCreature.BP_LightCreature_C|SetLevelRef _output_get LevelReference)))