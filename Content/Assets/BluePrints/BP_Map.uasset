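; BP_Map tracks level zone completion and shadow-spawner lights within its MapCollision and triggers the game's finish screen.
; A one-second CheckingZones timer rescans overlapping actors, counts completed zones and the last active-light index, and copies the totals to BP_DarkSideCharacter.
; A parallel FZones timer derives the zone total and shows BP_FinishGame with UI-only input when that light value is zero after WorldTimer passes ten seconds.
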(event Custom|CheckingZones
  (bind _mapcollision (Variables|Default|GetMapCollision))
  (Utilities|Array|Clear (Variables|Default|GetZones))
  (Utilities|Array|Clear (Variables|Default|GetLights))
  (for _array_element (Collision|GetOverlappingActors _mapcollision "/Game/AI/BP_ShadowSpawner.BP_ShadowSpawner_C" :!class /Script/Engine.PrimitiveComponent)
    (bind _asbp_shadow_spawner (Utilities|Casting|CastToBP_ShadowSpawner _array_element))
    (if (Variables|/Game/AI/BP_ShadowSpawner.BP_ShadowSpawner_C|GetIsActive _asbp_shadow_spawner)
      (bind _returnvalue (Utilities|Array|Add (Variables|Default|GetLights) _asbp_shadow_spawner))
      (Variables|Default|SetActiveMaxLights _returnvalue)
      (else
        (bind _returnvalue_2 (Utilities|Array|Add (Variables|Default|GetInactiveLights) _asbp_shadow_spawner))
        (Variables|Default|SetInactiveMaxLights (- _returnvalue_2 1)))))
  (for _array_element_2 (Collision|GetOverlappingActors _mapcollision "/Game/Assets/BluePrints/BP_Level.BP_Level_C" :!class /Script/Engine.PrimitiveComponent)
    (bind _asbp_level (Utilities|Casting|CastToBP_Level _array_element_2))
    (Utilities|Array|Add (Variables|Default|GetZones) _asbp_level))
  (Variables|Default|SetCompleted%20Zones 0)
  (for _array_element_3 (Variables|Default|GetZones)
    (bind _asbp_level_2 (Utilities|Casting|CastToBP_Level _array_element_3))
    (if (Variables|/Game/Assets/BluePrints/BP_Level.BP_Level_C|GetIsCompleted _asbp_level_2)
      (bind _output_get (Variables|Default|SetCompleted%20Zones (+ (Variables|Default|GetCompleted%20Zones) 1))))
    (Variables|Default|SetZonesRemaining (- (Variables|Default|GetAllZones) _output_get))
    (bind _asbp_dark_side_character (Utilities|Casting|CastToBP_DarkSideCharacter (Game|GetPlayerCharacter 0)))
    (Variables|/Game/PC/BP_DarkSideCharacter.BP_DarkSideCharacter_C|SetAllZones _asbp_dark_side_character (Variables|Default|GetAllZones))
    (Variables|/Game/PC/BP_DarkSideCharacter.BP_DarkSideCharacter_C|SetCompletedZones _asbp_dark_side_character (Variables|Default|GetCompleted%20Zones))
    (Variables|/Game/PC/BP_DarkSideCharacter.BP_DarkSideCharacter_C|SetZonesRemaining _asbp_dark_side_character (Variables|Default|GetZonesRemaining))
    (if (== (Variables|Default|GetActiveMaxLights) 0)
      (Variables|Default|SetZonesRemaining 0))
    (Variables|/Game/PC/BP_DarkSideCharacter.BP_DarkSideCharacter_C|SetTotalActiveLights _asbp_dark_side_character (Math|Conversions|ToFloat(Integer) (Variables|Default|GetActiveMaxLights)))))

(event Custom|FZones
  (if (Collision|IsOverlappingActor (Variables|Default|GetMapCollision) (stale Custom|CheckingZones _asbp_level) :!class /Script/Engine.PrimitiveComponent)
    (for _index (range 0 (+ (Utilities|Array|Length (Variables|Default|GetZones)) 1))
      (Variables|Default|SetAllZones (- _index 1))
      (if (> (Variables|/Game/PC/BP_DarkSidePlayerController.BP_DarkSidePlayerController_C|GetWorldTimer (stale _asbp_dark_side_player_controller)) 1e+01)
        (if (== (Variables|Default|GetActiveMaxLights) 0)
          (Variables|Default|SetZonesRemaining 0)
          (bind _asbp_dark_side_player_controller (Utilities|Casting|CastToBP_DarkSidePlayerController (Game|GetPlayerController 0)))
          (bind _returnvalue (UserInterface|CreateWidget "/Game/UI/FinishGame/BP_FinishGame.BP_FinishGame_C" _asbp_dark_side_player_controller))
          (UserInterface|Viewport|AddtoViewport _returnvalue 0)
          (Input|SetInputModeUIOnly _asbp_dark_side_player_controller 0 "DoNotLock" false)
          (Variables|/Script/Engine.PlayerController|SetbShowMouseCursor _asbp_dark_side_player_controller true))))))

(event EventBeginPlay
  (Utilities|Time|SetTimerbyEvent (delegate Custom|CheckingZones) 1.0 true)
  (Utilities|Time|SetTimerbyEvent (delegate Custom|FZones) 1.0 true))

(event Collision|EventActorBeginOverlap
  (params (OtherActor :type Actor%20Object%20Reference)))

(event EventTick
  (params (DeltaSeconds :type Float%20%28single-precision%29)))

(fn ConstructionScript)